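; BaseGun is a gun actor that the first-person character picks up by overlap and fires as a hitscan weapon.
; On overlap it passes its class to the character's PickupGun, while the construction script removes the pickup Trigger from owned instances.
; useGun plays a sound, line-traces from the camera with persistent debug drawing, spawns an explosion at the hit location and calls PlayerHitMe on any AI character hit.
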(event Custom|useGun
  (bind _returnvalue (Game|GetPlayerCameraManager 0))
  (bind _returnvalue_2 (Transformation|GetActorLocation _returnvalue))
  ;[1 1 1] Raycast TIr
  (Audio|PlaySoundatLocation "/Game/FirstPerson/Audio/FirstPersonTemplateWeaponFire02.FirstPersonTemplateWeaponFire02" (Transformation|GetActorLocation)) ; Play firing sound
  (bind _outhit (Collision|LineTraceForObjects _returnvalue_2 (+ _returnvalue_2 (* (Transformation|GetActorForwardVector _returnvalue) 5e+03)) (Utilities|Array|MakeArray "ObjectTypeQuery1" "ObjectTypeQuery2" "ObjectTypeQuery3" "ObjectTypeQuery4" "ObjectTypeQuery5" "ObjectTypeQuery6") false 0 "Persistent"))
  (Effects|SpawnEmitteratLocation "/Game/StarterContent/Particles/P_Explosion.P_Explosion" (.Location (Collision|BreakHitResult _outhit)))
  (bind _asbase_aicharacter (Utilities|Casting|CastToBaseAICharacter (.HitActor (Collision|BreakHitResult _outhit))))
  (Default|PlayerHitMe _asbase_aicharacter))

(event EventBeginPlay)

(event EventActorBeginOverlap
  (params (OtherActor :type Actor%20Object%20Reference))
  ;[1 1 1] if player enter trigger, player pickup this gun
  (bind _asfirst_person_character (Utilities|Casting|CastToFirstPersonCharacter OtherActor))
  (bind _asactor (Utilities|Casting|CastToActorClass (Utilities|GetClass self)))
  (Default|PickupGun _asfirst_person_character _asactor))

(fn ConstructionScript
  ;[1 1 1] If owner is player, delete trigger
  (if (not (Utilities|Name|Equal(Name) (Utilities|String|StringToName (Utilities|GetObjectName (Components|GetOwner))) "None"))
    (Components|DestroyComponent (Variables|Default|GetTrigger))))