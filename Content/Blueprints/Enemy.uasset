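; Enemy actor that reacts to looking at the player by changing body color and firing after a cooldown.
; The construction script creates a dynamic material on the mesh, whose BodyColor switches between base and follow colors in LookAtPlayer and StopLookAtPlayer.
; Fire only plays a rifle animation and sound, ignoring its target; StopLookAtPlayer does not cancel a pending shot.
; PlayerHitMe is an empty stub, and nothing here triggers the look events.
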(event Custom|PlayerHitMe)

(event Custom|LookAtPlayer
  (Rendering|Material|SetVectorParameterValue (Variables|Default|GetdynaMat) "BodyColor" (Variables|Default|GetfollowColor) :!class /Script/Engine.MaterialInstanceDynamic)
  (Utilities|FlowControl|Delay (Variables|Default|GetfireCooldown))
  (CallFunction|Fire (Game|Player|GetPlayerPawn 0)))

(event Custom|StopLookAtPlayer
  (Rendering|Material|SetVectorParameterValue (Variables|Default|GetdynaMat) "BodyColor" (Variables|Default|GetbaseColor) :!class /Script/Engine.MaterialInstanceDynamic))

(event Custom|Fire
  (params (TargetPawn :type Pawn%20Object%20Reference))
  (bind _mesh (Variables|Character|GetMesh))
  (Components|Animation|PlayAnimation _mesh "/Game/AnimStarterPack/Fire_Rifle_Ironsights.Fire_Rifle_Ironsights" false)
  (Audio|PlaySoundatLocation "/Game/FirstPerson/Audio/FirstPersonTemplateWeaponFire02.FirstPersonTemplateWeaponFire02" (Transformation|GetWorldLocation _mesh)))

(event EventBeginPlay)

(event EventActorBeginOverlap
  (params (OtherActor :type Actor%20Object%20Reference)))

(event EventTick
  (params (DeltaSeconds :type Float%20%28single-precision%29)))

(fn ConstructionScript
  (bind _returnvalue (Rendering|Material|CreateDynamicMaterialInstance (Variables|Character|GetMesh) 0 0 :!class /Script/Engine.PrimitiveComponent))
  (bind _output_get (Variables|Default|SetdynaMat _returnvalue))
  (Rendering|Material|SetVectorParameterValue _output_get "BodyColor" (Variables|Default|GetbaseColor) :!class /Script/Engine.MaterialInstanceDynamic))